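; BP_AmmoPickupTest is a functional test that checks a character can pick up an ammo box into its inventory.
; Tick drives the character forward with movement input every frame, and StartTest binds a check to the ammo box's picked-up event.
; When that event fires, the test succeeds if the inventory returns that same box; the graph has no explicit failure branch.
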(event Custom|CheckAmmoboxInInventory
  (bind _ammobox (Variables|Default|GetAmmoBox))
  (bind _returnvalue (Class|UInventoryComponent|FindSpecificItem (Variables|/Script/UE4CCP_Assignment1.UE4CCP_Assignment1Character|GetInventory (Variables|Default|GetCharacter)) _ammobox))
  (if (== _returnvalue _ammobox)
    (Class|FunctionalTest|FinishTest "Succeeded" "Ammo box was picked up.")))

(event EventPrepareTest)

(event EventStartTest
  (EventDispatchers|BindEventtoAmmoboxPickedUp (Variables|Default|GetAmmoBox) (delegate Custom|CheckAmmoboxInInventory)))

(event EventTick
  (params (DeltaSeconds :type Float%20%28single-precision%29))
  (bind _character (Variables|Default|GetCharacter))
  (Pawn|Input|AddMovementInput _character (Transformation|GetActorForwardVector _character) 1.0 false))

(fn ConstructionScript)