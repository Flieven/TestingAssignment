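; BP_LinetraceAmmoBox is an ammo box pickup for linetrace ammo that attaches to the player character on overlap.
; OnOverlap disables physics, attaches and snaps the box to the first-person mesh's GripPoint.
; It becomes the character's EquippedObject if none is valid, otherwise it is hidden with tick disabled.
; Simple accessors expose capacity, ammo type and current ammo, and an event sets the current amount.
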(event EventBeginPlay
  (|CallParentFunction))

(event Collision|EventActorBeginOverlap
  (params (OtherActor :type Actor%20Object%20Reference))
  (|CallParentFunction OtherActor) ; This node is disabled and will not be called.\nDrag off pins to build functionality.
)

(event EventOnOverlap
  (params (Caller :type Actor%20Object%20Reference))
  (bind _asue4ccp_assignment_1character (Utilities|Casting|CastToUE4CCP_Assignment1Character Caller))
  (Physics|SetSimulatePhysics (Variables|Default|GetSphereCollider) false)
  (Transformation|AttachComponentToComponent (Variables|/Script/UE4CCP_Assignment1.UE4CCP_Assignment1Character|GetMesh1P _asue4ccp_assignment_1character) "GripPoint" "SnapToTarget" "SnapToTarget" "SnapToTarget" true)
  (Transformation|SetActorLocation (Transformation|GetSocketLocation (Variables|/Script/UE4CCP_Assignment1.UE4CCP_Assignment1Character|GetMesh1P _asue4ccp_assignment_1character) "GripPoint") false true)
  (if (Utilities|IsValid (Variables|/Script/UE4CCP_Assignment1.UE4CCP_Assignment1Character|GetEquippedObject _asue4ccp_assignment_1character))
    (Rendering|SetActorHiddenInGame true)
    (Actor|Tick|SetActorTickEnabled false)
    (else
      (Variables|/Script/UE4CCP_Assignment1.UE4CCP_Assignment1Character|SetEquippedObject _asue4ccp_assignment_1character self)
      (Rendering|SetActorHiddenInGame false)
      (Actor|Tick|SetActorTickEnabled true))))

(event EventSetCurrentAmmo
  (params (Amount :type Integer))
  (Variables|Default|SetCurrentAmmo Amount))

(fn ConstructionScript
  (|CallParentFunction))

(fn GetAmmoCapacity
  (return (Variables|Default|GetAmmoCapacity)))

(fn GetCurrentAmmo
  (return (Variables|Default|GetCurrentAmmo)))

(fn GetAmmoType
  (return "/Game/Weapons/Ammo/Linetraceammo.Linetraceammo"))